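; BP_PlayerManager is a manager for the walking game that spawns and possesses the player character.
; Its Inialize event calls SpawnPlayer, which spawns BP_WalkingCharacterNew and has player controller 0 possess it.
; The spawn transform comes from FindPlayerStart, which takes the first valid PlayerStart in the level and prints a message for any invalid one it encounters.
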(event `/Game/WalkingGame/Modes/Interface/BPI_Initalize.Inialize`
  (`self.SpawnPlayer`))

(fn `FindPlayerStart`
  (returns (`Player Start` :type "Transform Structure"))
  (bind _outactors (`GameplayStatics.GetAllActorsOfClass` "/Script/Engine.PlayerStart"))
  (for _array_element _outactors
    (`/Engine/EditorBlueprintResources/StandardMacros.IsValid` _array_element
      (:`Is Valid`
        (set `self.PlayerStartTransform` (`self.GetTransform` _array_element))
        (break))
      (:`Is Not Valid`
        (`KismetSystemLibrary.PrintString` "Player Start Not Valid"))))
  (return (`self.PlayerStartTransform`)))

(fn `SpawnPlayer`
  (bind _player_start (`self.FindPlayerStart`))
  (bind _returnvalue (`|SpawnActorFromClass` "/Game/WalkingGame/Character/BP_WalkingCharacterNew.BP_WalkingCharacterNew_C" _player_start "Undefined" "MultiplyWithRoot" null null))
  (`Controller.Possess` (`GameplayStatics.GetPlayerController` 0) _returnvalue))

(fn `UserConstructionScript`
  (`parent.UserConstructionScript`))