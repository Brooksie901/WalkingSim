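; BP_WalkingGamemode is the game mode for the walking game, stepping through Initalize, PreGameStart, StartGame and EndGame states from BeginPlay.
; ChangeGameState switches on a state value to call the matching event; each state chains straight into the next, with only debug prints beyond initialization.
; Initalize uses SetUpManager to find the level's player and puzzle managers and send them InializeMessage, printing an error if one is missing.
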(event `self.ReceiveBeginPlay`
  (`/Game/WalkingGame/Modes/Interface/BPI_ChangeGameState.Change Game State` "NewEnumerator0"))

(event `Initalize`
  (`KismetSystemLibrary.PrintString` "Initalize")
  (`self.SetUp Manager` "/Game/WalkingGame/Modes/Managers/BP_PlayerManager.BP_PlayerManager_C")
  (`self.SetUp Manager` "/Game/WalkingGame/Modes/Managers/BP_PuzzleManager.BP_PuzzleManager_C")
  (`/Game/WalkingGame/Modes/Interface/BPI_ChangeGameState.Change Game State` "NewEnumerator1"))

(event `Pre Game Start`
  (`KismetSystemLibrary.PrintString` "Pre Game Start")
  (`/Game/WalkingGame/Modes/Interface/BPI_ChangeGameState.Change Game State` "NewEnumerator2"))

(event `Start Game`
  (`KismetSystemLibrary.PrintString` "Start Game")
  (`/Game/WalkingGame/Modes/Interface/BPI_ChangeGameState.Change Game State` "NewEnumerator3"))

(event `End Game`
  (`KismetSystemLibrary.PrintString` "End Game"))

(event `/Game/WalkingGame/Modes/Interface/BPI_ChangeGameState.Change Game State`
  (params (`Game State` :type "/Game/WalkingGame/Modes/Enum_GameStates Enum" :default "NewEnumerator0"))
  (switch `/Game/WalkingGame/Modes/Enum_GameStates` `Game State`
    (:`NewEnumerator0`
      (`self.Initalize`))
    (:`NewEnumerator1`
      (`self.Pre Game Start`))
    (:`NewEnumerator2`
      (`self.Start Game`))
    (:`NewEnumerator3`
      (`self.End Game`))))

(fn `ChangeGameState`)

(fn `SetUp Manager`
  (params (`Manager Class Type` :type "/Game/WalkingGame/Modes/Managers/BP_Manager Class Reference"))
  (locals (TempManagerRef :type "/Game/WalkingGame/Modes/Managers/BP_Manager Object Reference"))
  (bind _returnvalue (`GameplayStatics.GetActorOfClass` `Manager Class Type`))
  (bind _output_get (set `local.TempManagerRef` _returnvalue))
  (`/Engine/EditorBlueprintResources/StandardMacros.IsValid` _output_get
    (:`Is Valid`
      (message `/Game/WalkingGame/Modes/Interface/BPI_Initalize.Inialize` (`local.TempManagerRef`)))
    (:`Is Not Valid`
      (`KismetSystemLibrary.PrintString` (`KismetStringLibrary.Concat_StrStr` "Error: Manager of type (" (`KismetSystemLibrary.GetClassDisplayName` (`local.Manager Class Type`)) ") is not in level") true true (struct :`R` 1.0 :`G` 0.053658 :`A` 1.0)))))

(fn `UserConstructionScript`)