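; BP_WaterPillar is the Water pillar in the walking game's pillar puzzle.
; It handles the PillarTrigger event by switching on the pillar type and responds only to Water.
; On a match it prints a debug string and calls SetPillarComplete on the puzzle manager reference.
; BeginPlay and construction only call the parent, and overlap and tick are disabled.
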(event `self.ReceiveBeginPlay`
  (`parent.ReceiveBeginPlay`))

(event `/Game/WalkingGame/Blueprints/PillarPuzzle/Interface/BPI_PillarTrigger.PillarTrigger`
  (params (PillarType :type "/Game/WalkingGame/Blueprints/PillarPuzzle/Enum_PillarType Enum" :default "NewEnumerator0"))
  (switch `/Game/WalkingGame/Blueprints/PillarPuzzle/Enum_PillarType` PillarType
    (:`NewEnumerator0`
      (`KismetSystemLibrary.PrintString` "I am water")
      (`/Game/WalkingGame/Modes/Managers/BP_PuzzleManager.Set Pillar Complete` (`self.Puzzle ManagerRef`) "NewEnumerator0"))))

(fn `UserConstructionScript`
  (`parent.UserConstructionScript`))