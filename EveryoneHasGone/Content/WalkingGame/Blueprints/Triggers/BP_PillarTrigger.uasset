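; BP_PillarTrigger is an interactable trigger that reports its pillar type to a referenced pillar.
; Interacting through the interaction interface fires a DoOnce, so it sends PillarTriggerMessage with its PillarType to PillarRef only on the first interaction.
; The construction script writes the PillarType enum name onto a text render component as a visible label.
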(event `/Game/WalkingGame/Blueprints/Triggers/Interface/BPI_Interaction.Interact`
  ;[1 1 1] Interaction Interface Used for player Input
  (`/Engine/EditorBlueprintResources/StandardMacros.DoOnce` false
    (:`Completed`
      (message `/Game/WalkingGame/Blueprints/PillarPuzzle/Interface/BPI_PillarTrigger.PillarTrigger` (`self.PillarRef`) (`self.PillarType`)))))

(fn `UserConstructionScript`
  (`parent.UserConstructionScript`)
  (`TextRenderComponent.K2_SetText` (`self.TextRender`) (`KismetTextLibrary.Conv_StringToText` (`|GetEnumeratorNameAsString` (`self.PillarType`)))))